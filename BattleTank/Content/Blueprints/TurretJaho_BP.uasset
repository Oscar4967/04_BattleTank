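; Player-controlled turret Blueprint that aims and fires through a TurretAiming component.
; BeginPlay hands the barrel and dome to TurretAiming, and the Fire input calls its Fire.
; Axis inputs rotate the parts directly: AimAzimuth yaws TurretBarrel and AimElevation pitches TurretDome.
; Health bar setup is inactive: its call never runs and the function's widget logic is disconnected.
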(event `self.ReceiveBeginPlay`
  (`TankAimingComponent.Initialise` (`self.TurretAiming`) (`self.Turret Barrel`) (`self.Turret Dome`)))

(event `InputAction|Fire`
  (params (Key :type "Key Structure"))
  (:`Pressed`
    (`TankAimingComponent.Fire` (`self.TurretAiming`))))

(event `InputAxis|AimAzimuth`
  (params (AxisValue :type "Float (single-precision)"))
  (`SceneComponent.K2_AddLocalRotation` (`self.Turret Barrel`) (`KismetMathLibrary.MakeRotator` 0.0 0.0 AxisValue) false false))

(event `InputAxis|AimElevation`
  (params (AxisValue :type "Float (single-precision)"))
  (`SceneComponent.K2_AddLocalRotation` (`self.Turret Dome`) (`KismetMathLibrary.MakeRotator` 0.0 AxisValue) false false))

(fn `InitialiseHealthBarWidget`)

(fn `UserConstructionScript`)